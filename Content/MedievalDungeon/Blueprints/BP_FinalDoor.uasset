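; BP_FinalDoor is a key-locked double door that plays a locked sound until PickUpKey sets HasKey.
; With the key, Interact alternates between reversing and playing one timeline with close or open audio, starting on the reverse branch.
; The timeline lerps both leaves' yaw in opposite directions, using a FlipFlop that updates one leaf per tick.
; The unlock sound is an unfinished to-do.
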(event EventInteract
  (bind _sc_heavydooropen (Variables|Default|GetSC_HeavyDoorOpen))
  (bind _sc_heavydoorclose (Variables|Default|GetSC_HeavyDoorClose))
  ;[1 1 1] Interact
  (if (Variables|Default|GetHasKey?)
    (Utilities|FlowControl|FlipFlop
      (:A
        ;;[1 1 1] Audio
        ;;;[1 1 1] Door
        (Utilities|FlowControl|Sequence
          (:then_0
            (bind _newtrack_0 (Timeline|OpenRTimeline Reverse)
              (:Update
                (Utilities|FlowControl|FlipFlop
                  (:A
                    (Transformation|SetRelativeRotation (Variables|Default|GetSM_DoorWay_Large_Door_Left) (Math|Rotator|MakeRotator 0.0 0.0 (Math|Float|Lerp 0.0 -9e+01 _newtrack_0)) false false))
                  (:B
                    (Transformation|SetRelativeRotation (Variables|Default|GetSM_DoorWay_Large_Door_Right) (Math|Rotator|MakeRotator 0.0 0.0 (Math|Float|Lerp 0.0 9e+01 _newtrack_0)) false false))))))
          (:then_1
            (Audio|Components|Audio|Stop _sc_heavydoorclose)
            (Audio|Components|Audio|Play _sc_heavydoorclose 0.0))))
      (:B
        (Audio|Components|Audio|Stop _sc_heavydooropen)
        (Audio|Components|Audio|Play _sc_heavydooropen 0.0)
        (Timeline|OpenRTimeline Play)))
    (else
      ;;;[1 1 1] KeyLockUnlock
      (Audio|Components|Audio|Play (Variables|Default|GetHeavyDoorLocked) 0.0))))

(event EventPickUpKey
  ;[1 1 1] Interact
  ;;[1 1 1] Key
  (Variables|Default|SetHasKey? true)
  (Audio|Components|Audio|Play (Variables|Default|GetPickUpItems) 0.0))

(fn ConstructionScript)