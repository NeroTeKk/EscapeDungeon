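; BP_Dungeon_Doorway is a dungeon double door that toggles open and closed each time its Interact event fires.
; A FlipFlop plays or reverses a Timeline, restarting the matching heavy-door open or close sound.
; The Timeline's track lerps the door leaves' yaw in opposite directions up to 90 degrees, with a second FlipFlop updating left and right on alternate ticks rather than together.
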(event EventInteract
  (bind _sc_heavydooropen (Variables|Default|GetSC_HeavyDoorOpen))
  (bind _sc_heavydoorclose (Variables|Default|GetSC_HeavyDoorClose))
  ;[1 1 1] Interact Door
  (Utilities|FlowControl|FlipFlop
    (:A
      ;;[1 1 1] Audio
      (Audio|Components|Audio|Stop _sc_heavydooropen)
      (Audio|Components|Audio|Play _sc_heavydooropen 0.0)
      (bind _newtrack_0 (Timeline|Timeline Play)
        (:Update
          (Utilities|FlowControl|FlipFlop
            (:A
              (Transformation|SetRelativeRotation (Variables|Default|GetSM_DoorWay_Large_Door_Left) (Math|Rotator|MakeRotator 0.0 0.0 (Math|Float|Lerp 0.0 -9e+01 _newtrack_0)) false false))
            (:B
              (Transformation|SetRelativeRotation (Variables|Default|GetSM_DoorWay_Large_Door_Right) (Math|Rotator|MakeRotator 0.0 0.0 (Math|Float|Lerp 0.0 9e+01 _newtrack_0)) false false))))))
    (:B
      (Utilities|FlowControl|Sequence
        (:then_0
          (Timeline|Timeline Reverse))
        (:then_1
          (Audio|Components|Audio|Stop _sc_heavydoorclose)
          (Audio|Components|Audio|Play _sc_heavydoorclose 0.0))))))

(fn ConstructionScript)