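; Interactive dungeon cell door that swings open and closed on alternate Interact calls.
; A FlipFlop plays or reverses a Timeline that lerps the door mesh's yaw.
; The door sound restarts immediately on opening and after a short delay on closing.
; An older overlap-driven version on a separate Door_Timeline remains, mostly disabled apart from the end-overlap reverse.
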(event OnComponentBeginOverlap(Box)
  (params (OverlappedComponent :type Primitive%20Component%20Object%20Reference) (OtherActor :type Actor%20Object%20Reference) (OtherComp :type Primitive%20Component%20Object%20Reference) (OtherBodyIndex :type Integer) (bFromSweep :type Boolean) (SweepResult :type Hit%20Result%20Structure%20%28by%20ref%29))
  (Utilities|Casting|CastToBP_FirstPersonCharacter OtherActor)
  (bind _doortime (Timeline|Door_Timeline Play)
    (:Update
      (Transformation|SetRelativeRotation (Variables|Default|GetSM_Cell_Door) (Math|Rotator|MakeRotator 0.0 0.0 (* _doortime 9e+01)) false false))))

(event OnComponentEndOverlap(Box)
  (params (OverlappedComponent :type Primitive%20Component%20Object%20Reference) (OtherActor :type Actor%20Object%20Reference) (OtherComp :type Primitive%20Component%20Object%20Reference) (OtherBodyIndex :type Integer))
  (Utilities|Casting|CastToBP_FirstPersonCharacter OtherActor)
  (bind _doortime (Timeline|Door_Timeline Reverse)
    (:Update
      (Transformation|SetRelativeRotation (Variables|Default|GetSM_Cell_Door) (Math|Rotator|MakeRotator 0.0 0.0 (* _doortime 9e+01)) false false))))

(event EventInteract
  (bind _sc_celldoor (Variables|Default|GetSC_CellDoor))
  ;[1 1 1] Interact_Door
  (Utilities|FlowControl|FlipFlop
    (:A
      ;;[1 1 1] AUDIO
      (Audio|Components|Audio|Stop _sc_celldoor)
      (Audio|Components|Audio|Play _sc_celldoor 0.0)
      (bind _doortime (Timeline|Timeline Play)
        (:Update
          (Transformation|SetRelativeRotation (Variables|Default|GetSM_Cell_Door) (Math|Rotator|MakeRotator 0.0 0.0 (Math|Float|Lerp 0.0 -1e+02 _doortime)) false false))))
    (:B
      (Utilities|FlowControl|Sequence
        (:then_0
          (Timeline|Timeline Reverse))
        (:then_1
          (Utilities|FlowControl|Delay 1.0)
          (Audio|Components|Audio|Stop _sc_celldoor)
          (Audio|Components|Audio|Play _sc_celldoor 0.0))))))

(fn ConstructionScript)